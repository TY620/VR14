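; BP_SwitchBox is a trigger switch that starts and stops several movement and timer objects through overlaps on its Cube component.
; Begin overlap sets IsPlay on the MoveLeftRight, MoveRect and Timer references and calls DoPlay on TimeLintLeftRight; end overlap clears the flags and calls DoStop.
; Both events print debug text and respond to any overlapping actor, with no filtering or overlap counting.
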(event OnComponentBeginOverlap(Cube)
  (params (OverlappedComponent :type Primitive%20Component%20Object%20Reference) (OtherActor :type Actor%20Object%20Reference) (OtherComp :type Primitive%20Component%20Object%20Reference) (OtherBodyIndex :type Integer) (bFromSweep :type Boolean) (SweepResult :type Hit%20Result%20Structure%20%28by%20ref%29))
  (Development|PrintString (Utilities|String|Append "overlapped" (Utilities|GetDisplayName OverlappedComponent) "Other Actor" (Utilities|GetDisplayName OtherActor) "Other Comp" (Utilities|GetDisplayName OtherComp)))
  (Variables|/Game/StartUnreal/BP_MoveLeftRight.BP_MoveLeftRight_C|SetIsPlay (Variables|Default|GetMoveLeftRight) true)
  (Default|DoPlay (Variables|Default|GetTimeLintLeftRight))
  (Variables|/Game/StartUnreal/BP_MoveRect.BP_MoveRect_C|SetIsPlay (Variables|Default|GetMoveRect) true)
  (Variables|/Game/StartUnreal/BP_Timer.BP_Timer_C|SetIsPlay (Variables|Default|GetTimer) true))

(event OnComponentEndOverlap(Cube)
  (params (OverlappedComponent :type Primitive%20Component%20Object%20Reference) (OtherActor :type Actor%20Object%20Reference) (OtherComp :type Primitive%20Component%20Object%20Reference) (OtherBodyIndex :type Integer))
  (Development|PrintString "Hello")
  (Variables|/Game/StartUnreal/BP_MoveLeftRight.BP_MoveLeftRight_C|SetIsPlay (Variables|Default|GetMoveLeftRight) false)
  (Default|DoStop (Variables|Default|GetTimeLintLeftRight))
  (Variables|/Game/StartUnreal/BP_MoveRect.BP_MoveRect_C|SetIsPlay (Variables|Default|GetMoveRect) false)
  (Variables|/Game/StartUnreal/BP_Timer.BP_Timer_C|SetIsPlay (Variables|Default|GetTimer) false))

(event EventBeginPlay)

(event Collision|EventActorBeginOverlap
  (params (OtherActor :type Actor%20Object%20Reference)))

(event EventTick
  (params (DeltaSeconds :type Float%20%28single-precision%29)))

(fn ConstructionScript)