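; BP_MoveRect is an actor that moves its Cube component around a square loop in the local X-Z plane while IsPlay is true.
; Each Tick, a switch on the MoveType enum nudges the cube right, up, left or down by a fixed step.
; When the cube's relative location passes that side's limit, MoveType advances to the next direction, forming a simple state machine.
; The step is per frame and not scaled by delta time, so speed follows frame rate.
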(event Collision|EventActorBeginOverlap
  (params (OtherActor :type Actor%20Object%20Reference)))

(event EventTick
  (params (DeltaSeconds :type Float%20%28single-precision%29))
  (if (Variables|Default|GetIsPlay)
    (switch Utilities|FlowControl|Switch|SwitchonEN_MoveType (Variables|Default|GetMoveType)
      (:NewEnumerator0
        (Transformation|AddRelativeLocation (Variables|Default|GetCube) (Math|Vector|MakeVector 1.0 0.0 0.0) false false)
        (if (> (.x (Variables|/Script/Engine.SceneComponent|GetRelativeLocation (Variables|Default|GetCube))) 1e+02)
          (Variables|Default|SetMoveType "NewEnumerator1")))
      (:NewEnumerator1
        (Transformation|AddRelativeLocation (Variables|Default|GetCube) (Math|Vector|MakeVector 0.0 0.0 1.0) false false)
        (if (> (.z (Variables|/Script/Engine.SceneComponent|GetRelativeLocation (Variables|Default|GetCube))) 1e+02)
          (Variables|Default|SetMoveType "NewEnumerator2")))
      (:NewEnumerator2
        (Transformation|AddRelativeLocation (Variables|Default|GetCube) (Math|Vector|MakeVector -1.0 0.0 0.0) false false)
        (if (< (.x (Variables|/Script/Engine.SceneComponent|GetRelativeLocation (Variables|Default|GetCube))) 0.0)
          (Variables|Default|SetMoveType "NewEnumerator3")))
      (:NewEnumerator3
        (Transformation|AddRelativeLocation (Variables|Default|GetCube) (Math|Vector|MakeVector 0.0 0.0 -1.0) false false)
        (if (< (.z (Variables|/Script/Engine.SceneComponent|GetRelativeLocation (Variables|Default|GetCube))) 0.0)
          (Variables|Default|SetMoveType "NewEnumerator0"))))))

(fn ConstructionScript)