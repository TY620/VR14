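; BP_Bullet is a physics-driven projectile actor that knocks back the third-person character it hits.
; On BeginPlay it launches its Sphere component forward with a large impulse, then destroys itself after a short delay.
; When the sphere hits a BP_ThirdPersonCharacter, it applies the inverted hit normal impulse to that character's CharacterMovement, without destroying the bullet on impact.
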(event OnComponentHit(Sphere)
  (params (HitComponent :type Primitive%20Component%20Object%20Reference) (OtherActor :type Actor%20Object%20Reference) (OtherComp :type Primitive%20Component%20Object%20Reference) (NormalImpulse :type Vector :default "0, 0, 0") (Hit :type Hit%20Result%20Structure%20%28by%20ref%29))
  (bind _asbp_third_person_character (Utilities|Casting|CastToBP_ThirdPersonCharacter OtherActor))
  (Physics|AddImpulse (Variables|/Script/Engine.Character|GetCharacterMovement _asbp_third_person_character) (* NormalImpulse -1.0) false))

(event EventBeginPlay
  (Physics|AddImpulse (Variables|Default|GetSphere) (* (Transformation|GetActorForwardVector) 2e+05) "None" false)
  (Utilities|FlowControl|Delay 5.0)
  (Actor|DestroyActor))

(event Collision|EventActorBeginOverlap
  (params (OtherActor :type Actor%20Object%20Reference)))

(event EventTick
  (params (DeltaSeconds :type Float%20%28single-precision%29)))

(fn ConstructionScript)